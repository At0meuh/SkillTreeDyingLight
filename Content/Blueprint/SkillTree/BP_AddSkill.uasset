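; BP_AddSkill is a trigger actor that grants the first-person character one skill, chosen by WhichSkill: Grappin, TarpinSolid or Sprint.
; The construction script labels its text render with the skill name at level 0.
; On box overlap, it calls the matching add-skill function on the character, then queries the SkillComponent and updates the label with the returned tier level.
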(event `self.ReceiveBeginPlay`)

(event `self.Box.OnComponentBeginOverlap`
  (params (OverlappedComponent :type "PrimitiveComponent Object Reference") (OtherActor :type "Actor Object Reference") (OtherComp :type "PrimitiveComponent Object Reference") (OtherBodyIndex :type Integer) (bFromSweep :type Boolean) (SweepResult :type "HitResult Structure (by ref)"))
  (bind (_success _tierlevel) (`/Game/Blueprint/SkillTree/SkillComponent.QuerySkill` (`/Game/Blueprint/FirstPerson/Blueprints/BP_FirstPersonCharacter.SkillComponent` (`self.PlayerRef`)) (`self.WhichSkill`) ""))
  (bind _asbp_first_person_character (cast `/Game/Blueprint/FirstPerson/Blueprints/BP_FirstPersonCharacter` OtherActor))
  (set `self.PlayerRef` _asbp_first_person_character)
  (switch `/Game/Blueprint/SkillTree/ESkills` (`self.WhichSkill`)
    (:`NewEnumerator0`
      (`/Game/Blueprint/FirstPerson/Blueprints/BP_FirstPersonCharacter.AddGrappinSkill` (`self.PlayerRef`)))
    (:`NewEnumerator1`
      (`/Game/Blueprint/FirstPerson/Blueprints/BP_FirstPersonCharacter.AddTarpinSolidSkill` (`self.PlayerRef`)))
    (:`NewEnumerator3`
      (`/Game/Blueprint/FirstPerson/Blueprints/BP_FirstPersonCharacter.AddSprintSkill` (`self.PlayerRef`))))
  (if _success
    (set `self.skillLevel` _tierlevel)
    (`TextRenderComponent.K2_SetText` (`self.TextRender`) (`|FormatText` "{SkillName} - Lvl {level} " (select `/Game/Blueprint/SkillTree/ESkills` (`self.WhichSkill`) :`NewEnumerator0` "Grappin" :`NewEnumerator1` "TarpinSolid" :`NewEnumerator3` "Sprint" :!type "Text") (`self.skillLevel`)))))

(fn `UserConstructionScript`
  (`TextRenderComponent.K2_SetText` (`self.TextRender`) (`|FormatText` "{SkillName} - Lvl 0" (select `/Game/Blueprint/SkillTree/ESkills` (`self.WhichSkill`) :`NewEnumerator0` "Grappin" :`NewEnumerator1` "TarpinSolid" :`NewEnumerator3` "Sprint" :!type "Text"))))