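; Skill component that records which skill-tree skills are unlocked and at what tier.
; AddSkill increments a skill's tier in the SkillUnlocks map, starting it at one on first unlock, and QuerySkill reports whether it is unlocked and its tier.
; Both functions key the map by an explicit row name, falling back to a hardcoded name selected from the Skill enum when none is given.
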(fn `AddSkill`
  (params (Skill :type "/Game/Blueprint/SkillTree/ESkills Enum" :default "NewEnumerator0") (RowName :type String))
  (locals (LocalRowName :type String))
  (bind (_value _returnvalue) (`BlueprintMapLibrary.Map_Find` (`self.SkillUnlocks`) (`local.LocalRowName`)))
  (if (not (`KismetStringLibrary.IsEmpty` RowName))
    (set `local.LocalRowName` RowName)
    (else
      (set `local.LocalRowName` (select `/Game/Blueprint/SkillTree/ESkills` Skill :`NewEnumerator0` "grappin" :`NewEnumerator1` "tarpin_solide"))))
  (if _returnvalue
    (`BlueprintMapLibrary.Map_Add` (`self.SkillUnlocks`) (`local.LocalRowName`) (+ _value 1))
    (return)
    (else
      (`BlueprintMapLibrary.Map_Add` (`self.SkillUnlocks`) (`local.LocalRowName`) 1)
      (return))))

(fn `QuerySkill`
  (params (Skill :type "/Game/Blueprint/SkillTree/ESkills Enum" :default "NewEnumerator0") (RowName :type String))
  (returns (Success :type Boolean) (TierLevel :type Integer))
  (locals (LocalRowName :type String))
  (bind (_value _returnvalue) (`BlueprintMapLibrary.Map_Find` (`self.SkillUnlocks`) (`local.LocalRowName`)))
  (if (not (`KismetStringLibrary.IsEmpty` RowName))
    (set `local.LocalRowName` RowName)
    (else
      (set `local.LocalRowName` (select `/Game/Blueprint/SkillTree/ESkills` Skill :`NewEnumerator0` "grappin" :`NewEnumerator1` "tarpin_solide"))))
  (if _returnvalue
    (return true _value)
    (else
      (return false 0))))